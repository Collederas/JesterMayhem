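; Health component that lets its owning actor take damage and die.
; On BeginPlay it binds to the owner's OnTakeAnyDamage and sets health to maximum, then subtracts incoming damage from it.
; Non-lethal hits spawn an attached explosion emitter and a hit sound, while the DamageFX variable goes unused.
; At zero or below, it spawns death effects and sound, broadcasts OnDead with the owner, then destroys that actor.
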(event `self.ReceiveBeginPlay`
  (add `Actor.OnTakeAnyDamage` (`self.GetOwner`) (delegate `OnTakeAnyDamage_Event`))
  (set `self.CurrentHealth` (`self.MaxHealth`)))

(event `OnTakeAnyDamage_Event`
  (params (DamagedActor :type "Actor Object Reference") (Damage :type "Float (single-precision)") (DamageType :type "DamageType Object Reference") (InstigatedBy :type "Controller Object Reference") (DamageCauser :type "Actor Object Reference"))
  (bind _output_get (set `self.CurrentHealth` (- (`self.CurrentHealth`) Damage)))
  (if (<= _output_get 0.0)
    (`self.Die`)
    (else
      (`GameplayStatics.SpawnEmitterAttached` "/Game/Particles/P_Explosion.P_Explosion" (`Actor.RootComponent` (`self.GetOwner`)))
      (`GameplayStatics.SpawnSoundAtLocation` (`self.HitSound`) (+ (`Actor.K2_GetActorLocation` DamagedActor) (0.0 0.0 100.0)) (struct) 1.0 1.0 0.0 null null))))

(event `Die`
  (bind _returnvalue (`self.GetOwner`))
  (bind _returnvalue_2 (`Actor.K2_GetActorLocation` (`self.GetOwner`)))
  (`NiagaraFunctionLibrary.SpawnSystemAtLocation` (`self.DeathFX`) _returnvalue_2)
  (`GameplayStatics.SpawnSoundAtLocation` (`self.DeathSound`) _returnvalue_2 (struct) 1.0 1.0 0.0 null null)
  (`self.OnDead` (`self.GetOwner`))
  (`/Engine/EditorBlueprintResources/StandardMacros.IsValid` _returnvalue
    (:`Is Valid`
      (`Actor.K2_DestroyActor` _returnvalue))))