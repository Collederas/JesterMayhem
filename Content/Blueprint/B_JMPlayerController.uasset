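; Player controller that handles input, movement and hitscan shooting for BP_JMPlayer and creates the HUD.
; On begin play it adds the default Enhanced Input mapping; on possess it caches the player and disables input on its death.
; Move and rotate inputs drive the pawn relative to control yaw.
; Holding shoot runs a looping timer that plays gunfire and sphere-traces along pawn forward to apply damage.
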(event `self.ReceiveBeginPlay`
  (`EnhancedInputSubsystemInterface.AddMappingContext` (subsystem `EnhancedInputLocalPlayerSubsystem`) "/Game/Input/IMC_Default.IMC_Default" 0 (struct))
  (bind _returnvalue (`|CreateWidget` "/Game/UI/W_HUD.W_HUD_C" self))
  (`UserWidget.AddToViewport` _returnvalue 0))

(event `self.ReceivePossess`
  (params (PossessedPawn :type "Pawn Object Reference"))
  (bind _asbp_jmplayer (cast `/Game/Characters/Player/BP_JMPlayer` PossessedPawn))
  (bind _output_get (set `self.PlayerRef` _asbp_jmplayer))
  (add `/Game/Characters/Player/BP_JMPlayer.OnDeath` _output_get (delegate `OnDeath_Event`)))

(event `OnDeath_Event`
  (`self.DisableInput` self))

(event `EnhancedInput|/Game/Input/Actions/IA_Shoot`
  (params (ActionValue :type Boolean) (ElapsedSeconds :type "Float (double-precision)") (TriggeredSeconds :type "Float (double-precision)") (InputAction :type "InputAction Object Reference" :default "/Game/Input/Actions/IA_Shoot.IA_Shoot"))
  (:`Triggered`
    (bind _returnvalue (`KismetSystemLibrary.K2_SetTimerDelegate` (delegate `Fire`) (`self.FireRate`) true -1.0))
    (set `self.FiringTimer` _returnvalue))
  (:`Completed`
    (`KismetSystemLibrary.K2_ClearAndInvalidateTimerHandle` (`self.FiringTimer`))))

(event `EnhancedInput|/Game/Input/Actions/IA_Rotate`
  (params (ActionValue :type "Vector2D Structure") (ElapsedSeconds :type "Float (double-precision)") (TriggeredSeconds :type "Float (double-precision)") (InputAction :type "InputAction Object Reference" :default "/Game/Input/Actions/IA_Rotate.IA_Rotate"))
  (:`Triggered`
    (`self.AddYawInput` (* ActionValue_X (`self.TurnSpeed`)))))

(event `Fire`
  (bind _outlocation (`self.GetActorEyesViewPoint`))
  (`GameplayStatics.PlaySound2D` "/Game/Audio/SW_GunFire.SW_GunFire" 1.0 1.0 0.0 null null)
  (bind (_outhit _returnvalue) (`KismetSystemLibrary.SphereTraceSingleByProfile` _outlocation (+ _outlocation (* (`self.GetActorForwardVector` (`self.K2_GetPawn`)) (`self.ShootDistance`))) 20.0 "Pawn" false (`|MakeArray` (`self.K2_GetPawn`) :!type "Actor Object Reference") "ForDuration"))
  (if _returnvalue
    (`GameplayStatics.ApplyDamage` (`.HitActor` (`GameplayStatics.BreakHitResult` _outhit)) 10.0 self (`self.GetOwner`) "/Script/Engine.DamageType")))

(event `EnhancedInput|/Game/Input/Actions/IA_Move`
  (params (ActionValue :type "Vector2D Structure") (ElapsedSeconds :type "Float (double-precision)") (TriggeredSeconds :type "Float (double-precision)") (InputAction :type "InputAction Object Reference" :default "/Game/Input/Actions/IA_Move.IA_Move"))
  (bind (_returnvalue_roll _returnvalue_pitch _returnvalue_yaw) (`KismetMathLibrary.BreakRotator` (`self.GetControlRotation`)))
  (bind (_returnvalue_roll_2 _returnvalue_pitch_2 _returnvalue_yaw_2) (`KismetMathLibrary.BreakRotator` (`self.GetControlRotation`)))
  (:`Triggered`
    (`Pawn.AddMovementInput` (`self.PlayerRef`) (`KismetMathLibrary.GetRightVector` (`KismetMathLibrary.MakeRotator` _returnvalue_roll_2 0.0 _returnvalue_yaw_2)) ActionValue_X false)
    (`Pawn.AddMovementInput` (`self.PlayerRef`) (`KismetMathLibrary.GetForwardVector` (`KismetMathLibrary.MakeRotator` 0.0 0.0 _returnvalue_yaw)) ActionValue_Y false)))

(fn `UserConstructionScript`)